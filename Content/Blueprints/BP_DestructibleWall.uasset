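; BP_DestructibleWall is a wall that is destroyed after taking a random number of pick hits.
; BeginPlay rolls the required hit count and activates the wall's NavModifier.
; Each Destruct call increments the hit counter, and on reaching the threshold plays a sound, deactivates the NavModifier and destroys the actor.
; A physics and fracture-style collapse with delayed destruction is present but unconnected.
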(event Custom|Destruct
  (bind _result (Math|Integer|IncrementInt (Variables|Default|GetRecivedPicks))
    (:%20%20
      (if (>= _result (Variables|Default|GetPicksNeedsToDestruct))
        (Audio|PlaySound2D "/Game/SFX/FullDestructWall.FullDestructWall" 1.0 1.0 0.0 0 0)
        (Components|Activation|Deactivate (Variables|Default|GetNavModifier))
        (Actor|DestroyActor)))))

(event EventBeginPlay
  (Variables|Default|SetPicksNeedsToDestruct (Math|Random|RandomIntegerinRange 3 10))
  (Components|Activation|Activate (Variables|Default|GetNavModifier) true))

(fn ConstructionScript)