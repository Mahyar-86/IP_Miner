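; AI controller for the chaser enemy that runs BT_EnemyChaser and drives its blackboard state index.
; Hearing or flashlight-beam contact sets an investigate location (state 2), and sighting the player enters alert (state 3).
; During alert, Tick tracks player input as rage, escalating to state 4 at max rage or if the flashlight is lit.
; State 4 ignores new stimuli, while Tick also updates enemy feedback and player distance.
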(event OnPerceptionUpdated(AIPerception)
  (params (UpdatedActors :type Array%20of%20Actor%20Object%20References))
  (bind _blackboard (Variables|Default|GetBlackboard))
  (bind _blackboard_2 (Variables|Default|GetBlackboard))
  (for _array_element UpdatedActors
    (Utilities|FlowControl|Sequence
      (:then_0
        (bind (_sensed _stimulus) (CallFunction|CanSenseActor "NewEnumerator3" _array_element))
        (if _sensed
          (if (!= (Class|BlackboardComponent|GetValueasInt _blackboard_2 (Variables|Default|GetStationIndex%20Key%20)) 4)
            (AI|Components|Blackboard|SetValueasVector _blackboard_2 (Variables|Default|GetInvestigate%20Location%20Key) (.StimulusLocation (Utilities|Struct|BreakAIStimulus _stimulus)))
            (Class|BlackboardComponent|SetValueasInt _blackboard_2 (Variables|Default|GetStationIndex%20Key%20) 2))))
      (:then_1
        (bind _sensed_2 (CallFunction|CanSenseActor "NewEnumerator1" _array_element))
        (if _sensed_2
          (if (!= (Class|BlackboardComponent|GetValueasInt (Variables|Default|GetBlackboard) (Variables|Default|GetStationIndex%20Key%20)) 4)
            (bind _asbp_player (Utilities|Casting|CastToBP_Player _array_element))
            (Class|BlackboardComponent|SetValueasInt _blackboard (Variables|Default|GetStationIndex%20Key%20) 3)
            (bind _output_get (Variables|Default|SetAs%20BP%20First%20Person%20Character _asbp_player))
            (AI|Components|Blackboard|SetValueasVector _blackboard (Variables|Default|GetInvestigate%20Location%20Key) (Transformation|GetActorLocation _output_get))))))))

(event Custom|OnHasSeenLight
  (params (Light%20Location :type Vector))
  (bind _blackboard (Variables|Default|GetBlackboard))
  ;[0.07812 0.07812 0.07812 0.4435] Event Called when the enemy overlaped with the flashlights light
  (if (!= (Class|BlackboardComponent|GetValueasInt _blackboard (Variables|Default|GetStationIndex%20Key%20)) 4)
    (AI|Components|Blackboard|SetValueasVector _blackboard (Variables|Default|GetInvestigate%20Location%20Key) Light%20Location)
    (Class|BlackboardComponent|SetValueasInt _blackboard (Variables|Default|GetStationIndex%20Key%20) 2)))

(event EventTick
  (params (DeltaSeconds :type Float%20%28single-precision%29))
  (bind _returnvalue (Pawn|GetControlledPawn))
  (bind _as_bp_first_person_character (Variables|Default|GetAs%20BP%20First%20Person%20Character))
  (bind _as_bp_first_person_character_2 (Variables|Default|GetAs%20BP%20First%20Person%20Character))
  (bind _blackboard (Variables|Default|GetBlackboard))
  (bind _as_bp_first_person_character_3 (Variables|Default|GetAs%20BP%20First%20Person%20Character))
  (bind _blackboard_2 (Variables|Default|GetBlackboard))
  (bind _stationindex_key_ (Variables|Default|GetStationIndex%20Key%20))
  (bind _maxrage (Variables|Default|GetMaxRage))
  (bind _returnvalue_2 (Transformation|GetActorLocation _as_bp_first_person_character_2))
  (bind _returnvalue_3 (Transformation|GetActorLocation _returnvalue))
  (bind _returnvalue_4 (Class|BlackboardComponent|GetValueasInt _blackboard_2 _stationindex_key_))
  (bind _inputsofalertseenstate (Variables|/Game/Blueprints/BP_Player.BP_Player_C|GetInputsOfAlertSeenState _as_bp_first_person_character_3))
  (Utilities|FlowControl|Sequence
    (:then_0
      ;[0.06771 0.06771 0.06771 0.5] SetBehaviorTreeVariables
      (bind _asbp_enemy (Utilities|Casting|CastToBP_Enemy (Pawn|GetControlledPawn)))
      (Default|SetEnemysFeedacks _asbp_enemy _returnvalue_4)
      (if (== _returnvalue_4 3)
        (AI|Components|Blackboard|SetValueasObject _blackboard (Variables|Default|GetPlayer) _as_bp_first_person_character_3)
        (Default|StartListeningforInput _as_bp_first_person_character_3)
        (Default|CallOnRageChanged _maxrage _inputsofalertseenstate)
        (bind _asbp_flash_light (Utilities|Casting|CastToBP_FlashLight (Variables|/Script/Engine.ChildActorComponent|GetChildActor (Variables|/Game/Blueprints/BP_Player.BP_Player_C|GetBP_FlashLight _as_bp_first_person_character_3))))
        (if (or (>= _inputsofalertseenstate _maxrage) (Variables|/Game/Blueprints/BP_FlashLight.BP_FlashLight_C|GetIsLighting _asbp_flash_light))
          (Class|BlackboardComponent|SetValueasInt _blackboard (Variables|Default|GetStationIndex%20Key%20) 4)
          (Default|EndofListeningforMovement (Variables|Default|GetAs%20BP%20First%20Person%20Character)))
        (else
          (Utilities|IsValid _as_bp_first_person_character
            (:Is%20Valid
              (Default|EndofListeningforMovement _as_bp_first_person_character)
              (Default|CallOnRageChanged (Variables|Default|GetMaxRage) 0.0)
              (Variables|Default|SetShouldBroadCastAfterChangingState false))))))
    (:then_1
      ;[0.06771 0.06771 0.06771 0.5] Calculating Distance
      (Utilities|IsValid _as_bp_first_person_character_2
        (:Is%20Valid
          (AI|Components|Blackboard|SetValueasFloat (Variables|Default|GetBlackboard) (Variables|Default|GetDistance) (Math|Vector|Distance2D(Vector) (Math|Vector2D|MakeVector2D (.x _returnvalue_2) (.y _returnvalue_2)) (Math|Vector2D|MakeVector2D (.x _returnvalue_3) (.y _returnvalue_3)))))))))

(event EventPossess
  (params (PossessedPawn :type Pawn%20Object%20Reference))
  (AI|RunBehaviorTree "/Game/AI/BT_EnemyChaser.BT_EnemyChaser"))

(fn ConstructionScript)

(fn CanSenseActor
  (params (Sense :type E_EnemySenses%20Enum :default "NewEnumerator0") (SensedActor :type Actor%20Object%20Reference))
  (bind _info (Class|AIPerceptionComponent|GetActorsPerception (Variables|Default|GetAIPerception) SensedActor))
  (for _array_element (.LastSensedStimuli (Utilities|Struct|BreakActorPerceptionBlueprintInfo _info))
    (bind _returnvalue (Class|AIPerceptionSystem|GetSenseClassforStimulus _array_element))
    (if (== _returnvalue (Utilities|Select :Index Sense :NewEnumerator0 0 :NewEnumerator1 "/Script/AIModule.AISense_Sight" :NewEnumerator3 "/Script/AIModule.AISense_Hearing"))
      (return (.bSuccessfullySensed (Utilities|Struct|BreakAIStimulus _array_element)) _array_element))))