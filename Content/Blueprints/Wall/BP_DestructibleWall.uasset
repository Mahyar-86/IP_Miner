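; BP_DestructibleWall is a wall that breaks after a randomized number of pick hits.
; Each Destruct call decrements the count and broadcasts the remaining fraction, then plays a sound and destroys the actor at zero.
; Two WBP_WallProgressBar widgets receive a reference to the wall, and highlighting toggles custom-depth stencil rendering and child component visibility.
; A disconnected physics-based fracture sequence remains unused.
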(event Custom|UnHighLight
  (Rendering|SetRenderCustomDepth (Variables|Default|GetSM_UnbreakableWall) false)
  (Rendering|SetVisibility (Variables|Default|GetScene) false true))

(event Custom|Destruct
  (bind _result (Math|Integer|DecrementInt (Variables|Default|GetRecivedPicks))
    (:%20%20
      (Default|CallOnDestruction (/ _result (Variables|Default|GetPicksNeedsToDestruct)))
      (if (== _result 0)
        (Audio|PlaySound2D "/Game/Assets/SFX/FullDestructWall.FullDestructWall" 1.0 1.0 0.0 0 0)
        (Actor|DestroyActor)))))

(event Custom|HighLight
  (bind _sm_unbreakablewall (Variables|Default|GetSM_UnbreakableWall))
  (Rendering|SetRenderCustomDepth _sm_unbreakablewall true)
  (Rendering|SetCustomDepthStencilValue _sm_unbreakablewall 250)
  (Rendering|SetVisibility (Variables|Default|GetScene) true true))

(event EventBeginPlay
  (bind _output_get (Variables|Default|SetPicksNeedsToDestruct (Math|Random|RandomIntegerinRange 10 12)))
  (Variables|Default|SetRecivedPicks _output_get)
  (Rendering|SetRenderCustomDepth (Variables|Default|GetSM_UnbreakableWall) false)
  ;[0.15 0.15 0.15 0.5] Initialize Progressbar Widget
  (for _array_element (Utilities|Array|MakeArray (Variables|Default|GetProgressBar1) (Variables|Default|GetProgressBar))
    (bind _aswbp_wall_progress_bar (Utilities|Casting|CastToWBP_WallProgressBar (UserInterface|GetWidget _array_element)))
    (Variables|/Game/Blueprints/Widget/WBP_WallProgressBar.WBP_WallProgressBar_C|SetWall _aswbp_wall_progress_bar self)))

(fn ConstructionScript)