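; Laser emitter that projects a colored beam forward from its start body, stopping at whatever blocks it.
; On BeginPlay it applies LaserColor to the Laser effect's color parameter.
; Every Tick it line-traces on Visibility up to LongestDistance, ignoring itself, and feeds the distance to the impact point into the X of "Beam End".
; The trace's hit result is not checked before the impact point is used.
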(event EventBeginPlay
  (Effects|Components|ParticleSystem|SetColorParameter (Variables|Default|GetLaser) "Color" (Variables|Default|GetLaserColor)))

(event Collision|EventActorBeginOverlap
  (params (OtherActor :type Actor%20Object%20Reference)))

(event EventTick
  (params (DeltaSeconds :type Float%20%28single-precision%29))
  (bind _startbody (Variables|Default|GetStartBody))
  (bind _returnvalue (Transformation|GetWorldLocation _startbody))
  (bind _outhit (Collision|LineTraceByChannel _returnvalue (+ _returnvalue (* (Math|Vector|GetForwardVector _startbody) (Variables|Default|GetLongestDistance))) "TraceTypeQuery1" false (Utilities|Array|MakeArray self) "None"))
  (Effects|Components|ParticleSystem|SetVectorParameter (Variables|Default|GetLaser) "Beam End" (Math|Vector|MakeVector (Math|Vector|Distance(Vector) (Transformation|GetWorldLocation (Variables|Default|GetStartBody)) (.ImpactPoint (Collision|BreakHitResult _outhit))) 0.0 0.0)))

(fn ConstructionScript)