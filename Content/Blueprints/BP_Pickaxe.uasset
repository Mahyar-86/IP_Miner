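; BP_Pickaxe is the player's pickaxe, which breaks destructible walls and gives audio feedback when it hits walls.
; A trigger overlap only counts while the BP_Player pawn is picking, destroying BP_DestructibleWall actors or just playing a different sound for BP_NoneDestructibleWall.
; Either wall hit also makes the player character emit noise at the pickaxe's location through MakeNoise.
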(event OnComponentBeginOverlap(Trigger)
  (params (OverlappedComponent :type Primitive%20Component%20Object%20Reference) (OtherActor :type Actor%20Object%20Reference) (OtherComp :type Primitive%20Component%20Object%20Reference) (OtherBodyIndex :type Integer) (bFromSweep :type Boolean) (SweepResult :type Hit%20Result%20Structure%20%28by%20ref%29))
  (bind _asbp_player (Utilities|Casting|CastToBP_Player (Game|Player|GetPlayerPawn 0)))
  (if (Variables|/Game/Blueprints/BP_Player.BP_Player_C|GetbIsPicking _asbp_player)
    (bind _asbp_destructible_wall (Utilities|Casting|CastToBP_DestructibleWall OtherActor)
      (:then
        (Default|Destruct _asbp_destructible_wall)
        (CallFunction|DestructibleFeedback))
      (:CastFailed
        (Utilities|Casting|CastToBP_NoneDestructibleWall OtherActor)
        (CallFunction|NoneDestructibleFeedback)))
    (Class|Actor|MakeNoise (Game|GetPlayerCharacter 0) 1.0 0 (Transformation|GetActorLocation) 0.0 "None")))

(fn ConstructionScript)

(fn NoneDestructibleFeedback
  (Audio|PlaySound2D "/Game/Assets/SFX/PickingNoneDestructibleWall.PickingNoneDestructibleWall" 1.0 1.0 0.0 0 0))

(fn DestructibleFeedback
  (Audio|PlaySound2D "/Game/Assets/SFX/PickingDestructibleWall.PickingDestructibleWall" 1.0 1.0 0.0 0 0))